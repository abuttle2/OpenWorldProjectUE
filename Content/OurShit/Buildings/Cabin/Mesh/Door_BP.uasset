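; Cabin door Blueprint that toggles open and closed through an OpenDoor event, swinging away from or toward a side based on player position.
; On opening, the dot product of the player-to-door direction and the scene forward vector picks a positive or negative 90-degree yaw.
; A timeline lerps the door mesh's rotation and reverses to close, resetting the closed flag when finished.
; Tick prints the live dot product for debugging.
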(event `self.ReceiveBeginPlay`
  (bind _asbp_third_person_character (cast `/Game/ThirdPerson/Blueprints/BP_ThirdPersonCharacter` (`GameplayStatics.GetPlayerCharacter` 0)))
  (set `self.PlayerRef` _asbp_third_person_character))

(event `OpenDoor`
  (bind _scene (`self.Scene`))
  (if (`self.isDoorClosed`)
    (set `self.isDoorClosed` false)
    (set `self.DotProduct` (`KismetMathLibrary.Dot_VectorVector` (`KismetMathLibrary.Normal` (- (`SceneComponent.K2_GetComponentLocation` _scene) (`self.K2_GetActorLocation` (`self.PlayerRef`)))) (`SceneComponent.GetForwardVector` _scene)))
    (bind (_direction _alpha) (`Timeline|OpenDoorTL` :!label _label)
      (:`Update`
        (`SceneComponent.K2_SetRelativeRotation` (`self.Cabin_Wood_Door`) (`KismetMathLibrary.MakeRotator` 0.0 0.0 (`KismetMathLibrary.Lerp` 0.0 (`KismetMathLibrary.SelectFloat` 90.0 -90.0 (>= (`self.DotProduct`) 0.0)) _alpha)) false false))
      (:`Finished`
        (switch `ETimelineDirection` _direction
          (:`Backward`
            (set `self.isDoorClosed` true)))))
    (else
      (goto _label :!via `Reverse`))))

(event `self.ReceiveTick`
  (params (DeltaSeconds :type "Float (single-precision)"))
  (bind _scene (`self.Scene`))
  (`KismetSystemLibrary.PrintString` (`KismetStringLibrary.Conv_DoubleToString` (`KismetMathLibrary.Dot_VectorVector` (`KismetMathLibrary.Normal` (- (`SceneComponent.K2_GetComponentLocation` _scene) (`self.K2_GetActorLocation` (`self.PlayerRef`)))) (`SceneComponent.GetForwardVector` _scene))) true true (struct :`G` 0.66 :`B` 1.0 :`A` 1.0) DeltaSeconds))

(fn `UserConstructionScript`)