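; Modular shield actor that assembles its look from separate static mesh components, following customization choices held in BP_ThirdPersonGameMode.
; On BeginPlay it binds to the game mode's UI input event, which then swaps the base, pattern and trim meshes from the selected enums.
; The round trim shows only on round bases, otherwise it is cleared.
; Handle and boss logic, plus an older Construction Script version of the setup, are left disconnected.
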(event `self.ReceiveBeginPlay`
  (bind _asbp_third_person_game_mode (cast `/Game/ThirdPerson/Blueprints/BP_ThirdPersonGameMode` (`GameplayStatics.GetGameMode`)))
  (bind _output_get (set `self.As BP Third Person Game Mode` _asbp_third_person_game_mode))
  (add `/Game/ThirdPerson/Blueprints/BP_ThirdPersonGameMode.ED_UiInput` _output_get (delegate `CE_UiInput`)))

(event `CE_UiInput`
  (`|ExecutionSequence`
    (:`then_0`
      ;[1 1 1] Set Shield Base
      (switch `/Game/OurShit/CaiusTest/Shield/Blueprints/EN_Shield_Base` (`/Game/ThirdPerson/Blueprints/BP_ThirdPersonGameMode.ShieldType` (`self.As BP Third Person Game Mode`))
        (:`NewEnumerator0`
          (`StaticMeshComponent.SetStaticMesh` (`self.ShieldBase`) "/Game/OurShit/CaiusTest/Shield/Shield_Bases/Shield_Round_Planks_Hole.Shield_Round_Planks_Hole"))
        (:`NewEnumerator1`
          (`StaticMeshComponent.SetStaticMesh` (`self.ShieldBase`) "/Game/OurShit/CaiusTest/Shield/Shield_Bases/Shield_Round_Planks.Shield_Round_Planks"))
        (:`NewEnumerator2`
          (`StaticMeshComponent.SetStaticMesh` (`self.ShieldBase`) "/Game/PN_IvyPack/Meshes/staticBranches/2dBranch_01.2dBranch_01"))))
    (:`then_1`
      ;[1 1 1] Set Shield Pattern
      (switch `/Game/OurShit/CaiusTest/Shield/Blueprints/EN_Shield_Pattern` (`/Game/ThirdPerson/Blueprints/BP_ThirdPersonGameMode.ShieldPattern` (`self.As BP Third Person Game Mode`))
        (:`NewEnumerator3`
          (`StaticMeshComponent.SetStaticMesh` (`self.ShieldPattern`) null))
        (:`NewEnumerator0`
          (`StaticMeshComponent.SetStaticMesh` (`self.ShieldPattern`) "/Game/OurShit/CaiusTest/Shield/Shield_Patterns/Shield_Pattern_01.Shield_Pattern_01"))
        (:`NewEnumerator1`
          (`StaticMeshComponent.SetStaticMesh` (`self.ShieldPattern`) "/Game/OurShit/CaiusTest/Shield/Shield_Patterns/Shield_Pattern_02.Shield_Pattern_02"))
        (:`NewEnumerator2`
          (`StaticMeshComponent.SetStaticMesh` (`self.ShieldPattern`) "/Game/OurShit/CaiusTest/Shield/Shield_Patterns/Shield_Pattern_03.Shield_Pattern_03"))))
    (:`then_2`
      ;[1 1 1] Set Shield Trim
      (switch `/Game/OurShit/CaiusTest/Shield/Blueprints/EN_Shield_Trim` (`/Game/ThirdPerson/Blueprints/BP_ThirdPersonGameMode.ShieldTrim` (`self.As BP Third Person Game Mode`))
        (:`NewEnumerator0`
          (`StaticMeshComponent.SetStaticMesh` (`self.ShieldTrim`) null :!label _label))
        (:`NewEnumerator1`
          (if (or (`|EnumEquality` (`self.Selection`) "NewEnumerator1") (`|EnumEquality` (`self.Selection`) "NewEnumerator0"))
            (`StaticMeshComponent.SetStaticMesh` (`self.ShieldTrim`) "/Game/OurShit/CaiusTest/Shield/Shield_Trims/Shield_Round_trim_01.Shield_Round_trim_01")
            (else
              (set `self.Shield Trim` "NewEnumerator0")
              (goto _label))))))))

(fn `UserConstructionScript`)