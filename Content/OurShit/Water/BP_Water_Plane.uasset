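; BP_Water_Plane is a water surface actor that tiles a plane mesh into a flat rectangular grid.
; Its Construction Script adds local-space instances to the WaterPlane instanced mesh component, using MeshAmountX and MeshAmountY for tile counts and MeshLength and MeshWidth for spacing.
; The event graph holds only disabled placeholder events, so the actor runs no gameplay logic of its own.
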(fn `UserConstructionScript`
  (for _index (range (`self.MeshAmountX`))
    (for _index_2 (range (`self.MeshAmountY`))
      (`InstancedStaticMeshComponent.AddInstance` (`self.Water_Plane`) (`KismetMathLibrary.MakeTransform` (`KismetMathLibrary.MakeVector` (* _index (`self.MeshLength`)) (* _index_2 (`self.MeshWidth`)))) false))))